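; Health component for the player character that tracks health, armor and death, binding the owner's damage events on the server.
; Any-damage hits subtract health through an armor-based math expression, zero the armor and set Dead when health runs out.
; Point damage supplies shot direction to the damage-received dispatcher, with a flag guarding the directionless any-damage notification.
; OnRep Dead fires the death dispatcher, and debug prints remain.
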(event Custom|NotifyDamage
  (params (Damage :type Float%20%28single-precision%29) (DamageVector :type Vector))
  (Default|CallClientDamageRecieved Damage DamageVector))

(event Custom|OnPlayerTakeAnyDamage
  (params (DamagedActor :type Actor%20Object%20Reference) (Damage :type Float%20%28single-precision%29) (DamageType :type Damage%20Type%20Object%20Reference) (InstigatedBy :type Controller%20Object%20Reference) (DamageCauser :type Actor%20Object%20Reference))
  (bind _health (Variables|Default|GetHealth))
  (bind _returnvalue (<= _health 0.0))
  (if (CallFunction|ShouldbeDamaged InstigatedBy)
    (CallFunction|ApplyDamage Damage)
    (|Notifyanydamage Damage)
    (Development|PrintString (Utilities|String|ToString(Float) _health))
    (Development|PrintString (Utilities|String|ToString(Boolean) _returnvalue))
    (if _returnvalue
      (Variables|Default|SetDead true))))

(event Custom|OnPlayerTakePointDamage
  (params (DamagedActor :type Actor%20Object%20Reference) (Damage :type Float%20%28single-precision%29) (InstigatedBy :type Controller%20Object%20Reference) (HitLocation :type Vector) (FHitComponent :type Primitive%20Component%20Object%20Reference) (BoneName :type Name) (ShotFromDirection :type Vector) (DamageType :type Damage%20Type%20Object%20Reference) (DamageCauser :type Actor%20Object%20Reference))
  (if (CallFunction|ShouldbeDamaged InstigatedBy)
    (CallFunction|NotifyDamage Damage ShotFromDirection)
    (Variables|Default|SetDamageNotifyed true)))

(event EventBeginPlay
  (Variables|Default|SetHealth (Variables|Default|GetMaxHealth))
  (Variables|Default|SetArmor (Variables|Default|GetMaxArmor))
  (bind _asbp_player_character (Utilities|Casting|CastToBP_PlayerCharacter (Components|GetOwner)))
  (Variables|Default|SetCharacter _asbp_player_character)
  (if (Networking|IsServer)
    (EventDispatchers|BindEventtoOnTakeAnyDamage (Variables|Default|GetCharacter) (EventDispatchers|CreateEvent :!event Custom|OnPlayerTakeAnyDamage))
    (EventDispatchers|BindEventtoOnTakePointDamage (Variables|Default|GetCharacter) (EventDispatchers|CreateEvent :!event Custom|OnPlayerTakePointDamage))))

(fn OnRepDead
  (Development|PrintString "Dead")
  (Default|CallCharDead))

(fn ApplyDamage
  (params (Damage :type Float%20%28single-precision%29))
  (Variables|Default|SetHealth (- (Variables|Default|GetHealth) (|(Damage*(1-({95A674A0-4308-D671-68A6-6CA66E652994}/200))) Damage)))
  (Variables|Default|SetArmor 0.0)
  (return))

(fn GetHealth
  (return (Variables|Default|GetHealth) (Variables|Default|GetMaxHealth)))

(fn GetArmor
  (return (Variables|Default|GetArmor) (Variables|Default|GetMaxArmor)))

(fn ShouldbeDamaged
  (params (Object :type Object%20Object%20Reference))
  (if (Variables|Default|GetDead)
    (return false)
    (else
      (return true))))