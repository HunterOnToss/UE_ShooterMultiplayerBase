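; BP_WeaponManager is a player character component that manages weapon slots for main, secondary and melee weapons.
; CreateWeapon spawns a weapon owned by the player's controller, and AddWeapon slots it by type, making it current if none is set.
; A client-side RepNotify unhides the current weapon and attaches ClientWeaponAttached to the player.
; It also provides a camera interaction trace; ScrollWeapon is empty and DropWeapon only clears the first grenade's owner.
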(event `self.ReceiveBeginPlay`
  (bind _asbp_player_character (cast `/Game/Blueprints/Player/BP_PlayerCharacter` (`self.GetOwner`)))
  (set `self.Player` _asbp_player_character))

(fn `AddWeapon`
  (params (Weapon :type "/Game/Blueprints/Weapons/BP_Weapon Object Reference"))
  (locals (L_Weapon :type "/Game/Blueprints/Weapons/BP_Weapon Object Reference"))
  (bind _output_get (set `local.L_Weapon` Weapon))
  (bind _weapontype (`/Game/Blueprints/Weapons/BP_Weapon.WeaponType` _output_get))
  (`self.DropWeapon` (select `/Game/Data/Enum/E_WeaponType` _weapontype :`NewEnumerator0` (`self.MainWeapon`) :`NewEnumerator1` (`self.SecondWeapon`) :`NewEnumerator4` (`self.MeleeWeapon`)))
  (switch `/Game/Data/Enum/E_WeaponType` _weapontype
    (:`NewEnumerator0`
      (set `self.MainWeapon` (`local.L_Weapon`)))
    (:`NewEnumerator1`
      (set `self.SecondWeapon` (`local.L_Weapon`)))
    (:`NewEnumerator4`
      (set `self.MeleeWeapon` (`local.L_Weapon`))))
  (set `/Game/Blueprints/Weapons/BP_Weapon.WeaponOwner` (`self.Player`) (`local.L_Weapon`))
  (`self.CurrentWeapon`
    (:`then`)
    (:`else`
      (set `self.CurrentWeapon` (`local.L_Weapon`)))))

(fn `CreateWeapon`
  (params (Class :type "/Game/Blueprints/Weapons/BP_Weapon Class Reference"))
  (returns (Weapon :type "/Game/Blueprints/Weapons/BP_Weapon Object Reference"))
  (locals (L_Weapon :type "/Game/Blueprints/Weapons/BP_Weapon Object Reference"))
  (bind _player (`self.Player`))
  (bind _returnvalue (`|SpawnActorFromClass` Class (`KismetMathLibrary.MakeTransform` (0.0 0.0 0.0)) "AlwaysSpawn" "OverrideRootScale" (`Pawn.GetController` _player) _player _player))
  (bind _output_get (set `local.L_Weapon` _returnvalue))
  (`self.AddWeapon` _output_get)
  (return (`local.L_Weapon`)))

(fn `DropWeapon`
  (params (Weapon :type "/Game/Blueprints/Weapons/BP_Weapon Object Reference"))
  (locals (L_Weapon :type "/Game/Blueprints/Weapons/BP_Weapon Object Reference"))
  (set `/Game/Blueprints/Weapons/BP_Weapon.WeaponOwner` null (`|GetArrayItem` (`self.Grenades`))))

(fn `InteractTrace`
  (returns (Hit :type Boolean) (HitResult :type "HitResult Structure"))
  (bind _player (`self.Player`))
  (bind _returnvalue (`SceneComponent.K2_GetComponentLocation` (`/Game/Blueprints/Player/BP_PlayerCharacter.Camera` _player)))
  (bind (_outhit _returnvalue_2) (`KismetSystemLibrary.LineTraceSingle` _returnvalue (+ _returnvalue (* (`Actor.GetActorForwardVector` (`Pawn.GetController` _player)) 500.0)) "TraceTypeQuery1"))
  (return _returnvalue_2 _outhit))

(fn `OnRep_CurrentWeapon`
  (if (not (`KismetSystemLibrary.IsServer`))
    (bind _currentweapon (`self.CurrentWeapon`)
      (:`then`
        (`Actor.SetActorHiddenInGame` _currentweapon false)
        (bind _clientweaponattached (`self.ClientWeaponAttached`)
          (:`then`
            (`Actor.K2_AttachToActor` _clientweaponattached (`self.Player`) "None" "SnapToTarget" "SnapToTarget" "KeepRelative" true))
          (:`else`)))
      (:`else`
        (set `self.ClientWeaponAttached` null)))))

(fn `ScrollWeapon`
  (params (Next :type Boolean))
  (locals (L_Next :type Boolean) (L_Weapons :type "Array of /Game/Blueprints/Weapons/BP_Weapon Object Reference") (L_CurrentIndext :type Integer)))