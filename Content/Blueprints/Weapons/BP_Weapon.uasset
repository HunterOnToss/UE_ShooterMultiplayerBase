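; BP_Weapon is a weapon actor that characters pick up through Interact, which passes it to their weapon manager.
; UseWeapon spends ammo and locks firing behind a rate timer, whose callback fires again while auto-fire is active.
; The WeaponOwner RepNotify updates owner and collision, attaching the weapon on authority or detaching and revealing it when the owner is cleared.
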(fn `AbleToUse`
  (returns (Out :type Boolean))
  (return (and (> (`self.CurrentAmmo`) 0) (not (`self.UseFreezedByRate`)))))

(fn `Interact`
  (params (CharacterRef :type "/Game/Blueprints/Player/BP_PlayerCharacter Object Reference"))
  (returns (Success :type Boolean))
  (`/Game/Blueprints/Components/BP_WeaponManager.AddWeapon` (`/Game/Blueprints/Player/BP_PlayerCharacter.BP_WeaponManager` CharacterRef) self)
  (return false))

(fn `OnRep_WeaponOwner`
  (bind _weaponowner (`self.WeaponOwner`)
    (:`then`
      (bind _output_get (set `Actor.Instigator` null _weaponowner))
      (`self.SetOwner` (`Pawn.GetController` _output_get))
      (`self.SetActorEnableCollision` false)
      (`/Engine/EditorBlueprintResources/ActorMacros.Switch Has Authority`
        (:`Authority`
          (`self.K2_AttachToActor` (`self.WeaponOwner`) "None" "SnapToTarget" "SnapToTarget" "KeepRelative"))))
    (:`else`
      (`self.K2_DetachFromActor` "KeepRelative")
      (`self.SetActorHiddenInGame` false)
      (`self.SetActorEnableCollision` true)
      (`self.SetOwner` null))))

(fn `StopRateDelay`
  (set `self.UseFreezedByRate` false)
  (if (and (`self.FireActive`) (`self.AutoFire`))
    (`self.UseWeapon`)))

(fn `StopUseWeapon`
  (set `self.FireActive` false))

(fn `UserConstructionScript`)

(fn `UseWeapon`
  (returns (Used :type Boolean))
  (if (`self.AbleToUse`)
    (`/Engine/EditorBlueprintResources/StandardMacros.DecrementInt` (`self.CurrentAmmo`)
      (:`  `
        (`KismetSystemLibrary.K2_SetTimer` null "StopRateDelay" (`self.UseRate`))
        (set `self.UseFreezedByRate` true)
        (if (`self.AutoFire`)
          (set `self.FireActive` true))
        (return true)))
    (else
      (set `self.FireActive` false)
      (return false))))