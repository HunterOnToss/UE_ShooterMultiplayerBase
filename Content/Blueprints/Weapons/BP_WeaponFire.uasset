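; Weapon Blueprint that provides hitscan firing with random spread.
; ShootUsingTrace line-traces from the instigating player character's camera, applies point damage to the hit actor and passes the result to OnWeaponDamagedActor.
; GetShootDirection pitches the owner's forward vector by its look angle, then offsets it on two axes using a random stream within SpreadAngle.
; The event graph and Reloading RepNotify are empty.
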(fn `GetShootDirection`
  (returns (Direction :type "Vector Structure"))
  (bind _weaponowner (`self.WeaponOwner`))
  (bind _spreadangle (`self.SpreadAngle`))
  (bind _spreadangle_2 (`self.SpreadAngle`))
  (bind _returnvalue (`KismetMathLibrary.RotateAngleAxis` (`self.GetActorForwardVector` _weaponowner) (* (`/Game/Blueprints/Player/BP_PlayerCharacter.LookVerticalAngle` _weaponowner) -1.0) (`self.GetActorRightVector` _weaponowner)))
  (bind _returnvalue_2 (`KismetMathLibrary.Conv_VectorToRotator` _returnvalue))
  (return (`KismetMathLibrary.RotateAngleAxis` (`KismetMathLibrary.RotateAngleAxis` _returnvalue (`KismetMathLibrary.RandomFloatInRangeFromStream` (* _spreadangle_2 -1.0) _spreadangle_2 (`self.RandomStream`)) (`KismetMathLibrary.GetRightVector` _returnvalue_2)) (`KismetMathLibrary.RandomFloatInRangeFromStream` (* _spreadangle -1.0) _spreadangle (`self.RandomStream`)) (`KismetMathLibrary.GetUpVector` _returnvalue_2))))

(fn `OnRep_Reloading`)

(fn `ShootUsingTrace`
  (locals (L_Direction :type "Vector Structure" :default (0.0 0.0 0.0)))
  (bind _asbp_player_character (cast `/Game/Blueprints/Player/BP_PlayerCharacter` (`self.GetInstigator`))
    (:`then`
      (set `local.L_Direction` (`self.GetShootDirection`))
      (bind _returnvalue (`SceneComponent.K2_GetComponentLocation` (`/Game/Blueprints/Player/BP_PlayerCharacter.Camera` _asbp_player_character)))
      (bind _outhit (`KismetSystemLibrary.LineTraceSingleForObjects` _returnvalue (+ _returnvalue (* (`local.L_Direction`) 10000.0)) (`|MakeArray` "ObjectTypeQuery1" "ObjectTypeQuery2" "ObjectTypeQuery3" :!type "EObjectTypeQuery Enum") false (`|MakeArray` self (`self.GetInstigator`) :!type "Actor Object Reference")))
      (bind (_bblockinghit _binitialoverlap _time _distance _location _impactpoint _normal _impactnormal _physmat _hitactor _hitcomponent _hitbonename _hititem _faceindex _tracestart _traceend) (`GameplayStatics.BreakHitResult` _outhit))
      (bind _returnvalue_2 (`GameplayStatics.ApplyPointDamage` _hitactor (`self.Damage`) (`KismetMathLibrary.GetDirectionUnitVector` _tracestart _traceend) _outhit (`self.GetInstigatorController`) self))
      (`self.OnWeaponDamagedActor` _returnvalue_2 _hitactor)
      (return))
    (:`CastFailed`
      (return))))

(fn `UserConstructionScript`
  (`parent.UserConstructionScript`))